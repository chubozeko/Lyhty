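; BP_StaffOnly is a proximity-triggered "staff only" notice that appears when the first-person player approaches.
; The text component starts hidden on BeginPlay.
; BoxCollider overlap events, filtered to BP_FirstPersonCharacter, show the text and play an audio component on entry, then hide the text on exit.
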(event OnComponentBeginOverlap(BoxCollider)
  (params (OverlappedComponent :type Primitive%20Component%20Object%20Reference) (OtherActor :type Actor%20Object%20Reference) (OtherComp :type Primitive%20Component%20Object%20Reference) (OtherBodyIndex :type Integer) (bFromSweep :type Boolean) (SweepResult :type Hit%20Result%20Structure%20%28by%20ref%29))
  (Utilities|Casting|CastToBP_FirstPersonCharacter OtherActor)
  (Rendering|SetVisibility (Variables|Default|Gettxt_StaffOnly) true false)
  (Audio|Components|Audio|Play (Variables|Default|GetAudio) 0.0))

(event OnComponentEndOverlap(BoxCollider)
  (params (OverlappedComponent :type Primitive%20Component%20Object%20Reference) (OtherActor :type Actor%20Object%20Reference) (OtherComp :type Primitive%20Component%20Object%20Reference) (OtherBodyIndex :type Integer))
  (Utilities|Casting|CastToBP_FirstPersonCharacter OtherActor)
  (Rendering|SetVisibility (Variables|Default|Gettxt_StaffOnly) false false))

(event EventBeginPlay
  (Rendering|SetVisibility (Variables|Default|Gettxt_StaffOnly) false false))

(fn ConstructionScript)